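; Asteroid actor that drifts through the level and awards score when shot by a laser.
; Each tick nudges its static mesh along negative local X by a fixed step, not scaled by delta time.
; When its Sphere overlaps a Laser_Projectile, it adds its Score to the GameScore in LSDA_GameStateBase, then destroys both the projectile and itself.
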(event `self.ReceiveTick`
  (params (DeltaSeconds :type "Float (single-precision)"))
  ;[1 1 1] Movement
  (`SceneComponent.K2_AddLocalOffset` (`self.StaticMeshComponent`) (-0.5 0.0 0.0) false false))

(event `self.Sphere.OnComponentBeginOverlap`
  (params (OverlappedComponent :type "PrimitiveComponent Object Reference") (OtherActor :type "Actor Object Reference") (OtherComp :type "PrimitiveComponent Object Reference") (OtherBodyIndex :type Integer) (bFromSweep :type Boolean) (SweepResult :type "HitResult Structure (by ref)"))
  ;[1 1 1] Scoring
  (cast `/Game/Blueprints/Laser_Projectile` OtherActor)
  (bind _aslsda_game_state_base (cast `/Game/Blueprints/LSDA_GameStateBase` (`GameplayStatics.GetGameState`)))
  (set `/Game/Blueprints/LSDA_GameStateBase.GameScore` (+ (`self.Score`) (`/Game/Blueprints/LSDA_GameStateBase.GameScore` _aslsda_game_state_base)) _aslsda_game_state_base)
  (`self.K2_DestroyActor` OtherActor)
  (`self.K2_DestroyActor` (`ActorComponent.GetOwner` (`self.StaticMeshComponent`))))

(fn `UserConstructionScript`)