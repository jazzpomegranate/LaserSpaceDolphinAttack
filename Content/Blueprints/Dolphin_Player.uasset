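; Dolphin_Player is the player-controlled dolphin, which moves along one axis and fires laser projectiles.
; The Up-Down input axis offsets the Box component along its right vector, scaled by MovementSpeed, with a sweep for collision and no delta-time scaling.
; Pressing Shoot spawns a Laser_Projectile at the world transform of the ProjectileStart component.
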(event `InputAxis|Up-Down`
  (params (AxisValue :type "Float (single-precision)"))
  ;[1 1 1] Movement
  (`SceneComponent.K2_AddWorldOffset` (`self.Box`) (* (* (`SceneComponent.GetRightVector` (`self.Box`)) AxisValue) (`self.MovementSpeed`)) true false))

(event `InputAction|Shoot`
  (params (Key :type "Key Structure"))
  ;[1 1 1] Shooting
  (:`Pressed`
    (`|SpawnActorFromClass` "/Game/Blueprints/Laser_Projectile.Laser_Projectile_C" (`SceneComponent.K2_GetComponentToWorld` (`self.ProjectileStart`)) "Undefined" "OverrideRootScale" null null)))

(fn `UserConstructionScript`)